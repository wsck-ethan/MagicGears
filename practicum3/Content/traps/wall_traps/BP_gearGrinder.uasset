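; Gear grinder wall trap that damages non-hero actors entering its box trigger.
; On overlap it filters heroes out through a HeroMessage call, then waits for the trigger delay.
; If damage is allowed, it sends base damage to the actor via DamageTakenEventMessage, plays a 2D grinder sound and calls CooldownEvent.
; The target is not rechecked after the delay, so leaving the box does not prevent the hit.
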(event `self.Box_0.OnComponentBeginOverlap`
  (params (OverlappedComponent :type "PrimitiveComponent Object Reference") (OtherActor :type "Actor Object Reference") (OtherComp :type "PrimitiveComponent Object Reference") (OtherBodyIndex :type Integer) (bFromSweep :type Boolean) (SweepResult :type "HitResult Structure (by ref)"))
  (bind _hero (message `/Game/AI/BPI_baseStates.Hero` OtherActor))
  (if (not _hero)
    (`KismetSystemLibrary.Delay` (`self.trap trigger delay`))
    (if (`self.CanDamageTarget`)
      (message `/Game/AI/BPI_baseStates.damage taken  event  ` OtherActor (`self.base_damage`))
      (`GameplayStatics.PlaySound2D` "/Game/noise/Gear_Grinder_Trap_Mark_Up_1.Gear_Grinder_Trap_Mark_Up_1" 1.0 1.0 0.0 null null)
      (`self.cooldown Event`))))

(fn `UserConstructionScript`
  (`parent.UserConstructionScript`))