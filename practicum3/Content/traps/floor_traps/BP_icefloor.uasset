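; BP_icefloor is a floor trap that makes characters slide by altering their ground friction.
; Entering its box trigger sends minion and friction messages to the overlapping actor, setting both ground and braking friction negative, and plays an ice trap sound.
; Leaving the box sends the same messages with the stored base friction values to restore grip.
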(event `self.Box_0.OnComponentBeginOverlap`
  (params (OverlappedComponent :type "PrimitiveComponent Object Reference") (OtherActor :type "Actor Object Reference") (OtherComp :type "PrimitiveComponent Object Reference") (OtherBodyIndex :type Integer) (bFromSweep :type Boolean) (SweepResult :type "HitResult Structure (by ref)"))
  (message `/Game/AI/BPI_baseStates.minion` OtherActor)
  (message `/Game/AI/BPI_baseStates.CharaterGroundFriction` OtherActor -5.0 -5.0)
  (if true
    (`GameplayStatics.PlaySoundAtLocation` "/Game/noise/Ice_Trap.Ice_Trap" (`SceneComponent.K2_GetComponentLocation` (`self.DefaultSceneRoot`)) (struct) 1.0 1.0 0.0 null null null null)))

(event `self.Box_0.OnComponentEndOverlap`
  (params (OverlappedComponent :type "PrimitiveComponent Object Reference") (OtherActor :type "Actor Object Reference") (OtherComp :type "PrimitiveComponent Object Reference") (OtherBodyIndex :type Integer))
  (message `/Game/AI/BPI_baseStates.minion` OtherActor)
  (message `/Game/AI/BPI_baseStates.CharaterGroundFriction` OtherActor (`self.friction base number`) (`self.Braking Friction`)))

(fn `UserConstructionScript`
  (`parent.UserConstructionScript`))