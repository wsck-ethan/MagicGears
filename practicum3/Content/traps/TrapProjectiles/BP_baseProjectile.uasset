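; Base trap projectile that damages minions it overlaps.
; On overlap, an interface message identifies minions, then the projectile sends its Damage value, plays a sound, prints a debug string and destroys itself after a short delay.
; Identity and damage interface functions are stubs, reporting it as neither hero, minion nor attackable, with a fixed team and no damage response.
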(event `self.s.OnComponentBeginOverlap`
  (params (OverlappedComponent :type "PrimitiveComponent Object Reference") (OtherActor :type "Actor Object Reference") (OtherComp :type "PrimitiveComponent Object Reference") (OtherBodyIndex :type Integer) (bFromSweep :type Boolean) (SweepResult :type "HitResult Structure (by ref)"))
  (bind _minion (message `/Game/AI/BPI_baseStates.minion` OtherActor))
  (if _minion
    (message `/Game/AI/BPI_baseStates.damage taken  event  ` OtherActor (`self.damage`))
    (`AudioComponent.Play` (`self.Audio`) 0.0)
    (`KismetSystemLibrary.PrintString` "Hello")
    (`KismetSystemLibrary.Delay` 1.0)
    (`self.K2_DestroyActor`)))

(fn `attackable`
  (returns (attackable :type Boolean))
  (return false))

(fn `damage event `
  (params (`damage taken` :type Integer :default 0))
  (returns (`health actor` :type Integer))
  (return 0))

(fn `Hero`
  (returns (Hero :type Boolean))
  (return false))

(fn `minion`
  (returns (minion :type Boolean))
  (return false))

(fn `PointOfIntrest`
  (returns (`pointOfIntrest blue` :type "/Game/AI/pointOfIntrestFolder/BP_AIPointOfIntrest_blue Object Reference") (`pointOfIntrest red` :type "/Game/AI/pointOfIntrestFolder/BP_AIPointOfIntrest_red Object Reference"))
  (return null null))

(fn `TEAM`
  (returns (Team :type "/Game/AI/Enum/E_Team Enum"))
  (return "NewEnumerator0"))

(fn `UserConstructionScript`)