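; Roof cannon trap that shoots BP_baseProjectile at its current attack target and reports a fixed team.
; From BeginPlay, a short Delay loop repeatedly calls Fire, which acts only when a target exists and the cooldown has run out.
; Firing turns the Arrow component toward the target, spawns the projectile from its transform, then starts the cooldown.
; Target acquisition and cooldown logic are not defined in these graphs.
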(event `self.ReceiveBeginPlay`
  (`self.fire` :!label _label)
  (`KismetSystemLibrary.Delay` 0.01)
  (goto _label))

(event `fire`
  (if (`self.haveTarget`)
    (if (<= (`self.cooldown count`) 0)
      (`SceneComponent.K2_SetWorldRotation` (`self.Arrow`) (`KismetMathLibrary.FindLookAtRotation` (`self.K2_GetActorLocation`) (`self.K2_GetActorLocation` (`self.attackTarget`))) false false)
      (`|SpawnActorFromClass` "/Game/traps/TrapProjectiles/BP_baseProjectile.BP_baseProjectile_C" (`SceneComponent.K2_GetComponentToWorld` (`self.Arrow`)) "Undefined" "MultiplyWithRoot" null null)
      (`self.cooldown Event`))))

(fn `TEAM `
  (returns (Team :type "/Game/AI/Enum/E_Team Enum"))
  (return "NewEnumerator0"))

(fn `UserConstructionScript`
  (`parent.UserConstructionScript`))