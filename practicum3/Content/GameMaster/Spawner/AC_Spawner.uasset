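; Spawner component that runs data-driven enemy waves from DT_Waves.
; On BeginPlay it caches the player, the game master's object pool and all BP_EnemySpawner transforms.
; StartWave loads a row, then SpawnEnemy consumes entries after delays, spawning pooled enemies at indexed spawners; invalid indices use a cycling default, continuing only on wraparound.
; EndWave advances the index and readies the player, or prints a win once past the last wave.
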(event `self.ReceiveBeginPlay`
  (set `self.WaveIndex` 0)
  (bind _returnvalue (`GameplayStatics.GetActorOfClass` "/Game/ThirdPerson/Blueprints/BP_ThirdPersonCharacter.BP_ThirdPersonCharacter_C"))
  (set `self.Player` _returnvalue)
  (bind _returnvalue_2 (`GameplayStatics.GetActorOfClass` "/Game/GameMaster/BP_GameMaster.BP_GameMaster_C"))
  (set `self.ObjectPool` (`/Game/GameMaster/BP_GameMaster.AC_ObjectPool` _returnvalue_2))
  (bind _outrownames (`DataTableFunctionLibrary.GetDataTableRowNames` "/Game/GameMaster/Spawner/DT_Waves.DT_Waves"))
  (bind _output_get (set `self.Waves` _outrownames))
  (set `self.MaxWaves` (`KismetArrayLibrary.Array_Length` _output_get))
  (bind _outactors (`GameplayStatics.GetAllActorsOfClass` "/Game/GameMaster/Spawner/BP_EnemySpawner.BP_EnemySpawner_C"))
  (for _array_element _outactors
    (`KismetArrayLibrary.Array_Add` (`self.SpawnTransforms`) (`Actor.GetTransform` _array_element))))

(event `StartWave`
  (bind _waveindex (`self.WaveIndex`))
  (if (not (>= _waveindex (`self.MaxWaves`)))
    (bind _returnvalue (`|GetDataTableRow` "/Game/GameMaster/Spawner/DT_Waves.DT_Waves" (`|GetArrayItem` (`self.Waves`) _waveindex))
      (:`then`
        (bind _output_get (set `self.Enemies` (`KismetArrayLibrary.Array_Length` (break `/Game/GameMaster/Spawner/S_Wave` _returnvalue))))
        (`KismetSystemLibrary.PrintString` (`KismetStringLibrary.Conv_IntToString` _output_get))
        (set `self.WaveDataArray` (break `/Game/GameMaster/Spawner/S_Wave` _returnvalue))
        (`self.SpawnEnemy`)))))

(event `SpawnEnemy`
  (bind _wavedataarray (`self.WaveDataArray`))
  (bind _objectpool (`self.ObjectPool`))
  (bind _spawntransforms (`self.SpawnTransforms`))
  (bind _defaultspawnindex (`self.DefaultSpawnIndex`))
  (bind (_enemytype _spawndelay _spawnerindex) (break `/Game/GameMaster/Spawner/S_SpawnData` (`|GetArrayItem` (`self.WaveDataArray`))))
  (`KismetSystemLibrary.Delay` _spawndelay)
  (if (`KismetArrayLibrary.Array_IsValidIndex` _spawntransforms _spawnerindex)
    (bind _spawnedactor (`/Game/GameMaster/ObjectPooling/AC_ObjectPool.Spawn` _objectpool _enemytype (`|GetArrayItem` _spawntransforms _spawnerindex)))
    (message `/Game/GameMaster/ObjectPooling/BPI_ObjectPoolInterface.Active` _spawnedactor _objectpool (0.0 0.0 0.0))
    (`KismetArrayLibrary.Array_Remove` _wavedataarray :!label _label)
    (if (not (<= (`KismetArrayLibrary.Array_Length` _wavedataarray) 0))
      (`self.SpawnEnemy`))
    (else
      (bind _spawnedactor_2 (`/Game/GameMaster/ObjectPooling/AC_ObjectPool.Spawn` _objectpool _enemytype (`|GetArrayItem` _spawntransforms _defaultspawnindex)))
      (message `/Game/GameMaster/ObjectPooling/BPI_ObjectPoolInterface.Active` _spawnedactor_2 null (0.0 0.0 0.0))
      (bind _output_get (set `self.DefaultSpawnIndex` (+ _defaultspawnindex 1)))
      (if (not (`KismetArrayLibrary.Array_IsValidIndex` _spawntransforms _output_get))
        (set `self.DefaultSpawnIndex` 0)
        (goto _label)))))

(fn `EndGame`
  (`KismetSystemLibrary.PrintString` "You Win!"))

(fn `EndWave`
  (bind _waveindex (`self.WaveIndex`))
  (if (> _waveindex (`self.MaxWaves`))
    (`self.EndGame`)
    (else
      (`/Engine/EditorBlueprintResources/StandardMacros.IncrementInt` _waveindex
        (:`  `
          (set `/Game/ThirdPerson/Blueprints/BP_ThirdPersonCharacter.ReadyForNextWave` true (`self.Player`)))))))